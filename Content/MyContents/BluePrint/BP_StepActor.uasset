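; BP_StepActor is a step actor with a mesh and widget, whose empty StartStep and Interaction functions appear meant for child overrides.
; It binds to BP_GameState's state-change dispatcher, with CheckStep calling StartStep when the state matches MyStep.
; EndStep advances the game state to NextStep.
; Active and Passive show or hide the initially hidden widget, which a fast looping timer turns toward the player camera once activated.
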(event `self.ReceiveBeginPlay`
  (`self.BindFunction`)
  (`KismetSystemLibrary.K2_SetTimer` null "SetWidgetRotate" 0.01 true))

(fn `Active`
  (`self.SetWidget` true)
  (set `self.IsShowWidget` true))

(fn `BindFunction`
  (bind _asbp_game_state (cast `/MyContents/MyContents/BluePrint/BP_GameState` (`GameplayStatics.GetGameState`)))
  (add `/MyContents/MyContents/BluePrint/BP_GameState.NewEventDispatcher_ChangeState` _asbp_game_state (`|CreateDelegate` :!event `Check Step`)))

(fn `Check Step`
  (params (`Game State` :type "/MyContents/MyContents/BluePrint/EN_GameState Enum" :default "NewEnumerator0"))
  (if (`|EnumEquality` `Game State` (`self.MyStep`))
    (`self.StartStep`)))

(fn `EndStep`
  (bind _asbp_game_state (cast `/MyContents/MyContents/BluePrint/BP_GameState` (`GameplayStatics.GetGameState`)))
  (`/MyContents/MyContents/BluePrint/BP_GameState.ChangeState` _asbp_game_state (`self.NextStep`)))

(fn `Interaction`)

(fn `Passive`
  (`self.SetWidget` false))

(fn `SetWidget`
  (params (bNewVisibility :type Boolean))
  (`SceneComponent.SetVisibility` (`self.Widget`) bNewVisibility false))

(fn `SetWidgetRotate`
  (if (`self.IsShowWidget`)
    (`SceneComponent.K2_SetWorldRotation` (`self.Widget`) (`KismetMathLibrary.FindLookAtRotation` (`SceneComponent.K2_GetComponentLocation` (`self.Widget`)) (`self.K2_GetActorLocation` (`GameplayStatics.GetPlayerCameraManager` 0))) false false)))

(fn `StartStep`)

(fn `UserConstructionScript`
  (`StaticMeshComponent.SetStaticMesh` (`self.StaticMesh`) (`self.New Mesh`))
  (`SceneComponent.SetVisibility` (`self.Widget`) false false))